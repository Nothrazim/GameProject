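; Swinging door Blueprint that opens away from the first-person player on entering its trigger box, with end-overlap logic to close it.
; A dot product picks the opening direction, and a three-value state enum maps to target rotations, also applied in the Construction Script.
; TransitionToState uses a timeline to lerp the door mesh between rotations, guarding against overlapping transitions with a busy flag and a queued-request flag.
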(event `self.Box.OnComponentBeginOverlap`
  (params (OverlappedComponent :type "PrimitiveComponent Object Reference") (OtherActor :type "Actor Object Reference") (OtherComp :type "PrimitiveComponent Object Reference") (OtherBodyIndex :type Integer) (bFromSweep :type Boolean) (SweepResult :type "HitResult Structure (by ref)"))
  ;[1 1 1] On overlap, open door in opposite direction from where player is
  (`self.IsPlayer` OtherActor
    (:`isPlayer`
      (`/Engine/EditorBlueprintResources/StandardMacros.IsValid` null
        (:`Is Not Valid`
          (set `self.OverlappingPlayer` OtherActor)
          (`self.TransitionToState` (select `bool` (> (`self.GetDotProductTo` OtherActor) 0.0) :`false` "NewEnumerator1" :`true` "NewEnumerator2" :!type "/Game/GameProject/EDoorState Enum")))))))

(event `self.Box.OnComponentEndOverlap`
  (params (OverlappedComponent :type "PrimitiveComponent Object Reference") (OtherActor :type "Actor Object Reference") (OtherComp :type "PrimitiveComponent Object Reference") (OtherBodyIndex :type Integer))
  ;[1 1 1] On End overlap, close door
  (if (> (`KismetArrayLibrary.Array_Length` (`PrimitiveComponent.GetOverlappingActors` (`self.Box`) "/Game/FirstPersonBP/Blueprints/FirstPersonCharacter.FirstPersonCharacter_C")) 0)
    (`self.IsPlayer` OtherActor
      (:`isPlayer`
        (`/Engine/EditorBlueprintResources/StandardMacros.IsValid` (`self.OverlappingPlayer`)
          (:`Is Valid`
            (set `self.OverlappingPlayer` null)
            (`self.TransitionToState` "NewEnumerator0")))))))

(event `TransitionToState`
  (params (TargetState :type "/Game/GameProject/EDoorState Enum" :default "NewEnumerator0"))
  (if (and (`|EnumInequality` TargetState (`self.State`)) (not (`self.bTransitioning`)))
    (set `self.bStateQueued` false)
    (set `self.bTransitioning` true)
    (set `self.QueuedTargetState` TargetState)
    (bind (_direction _newtrack_0) (`Timeline|Timeline_0` :!via `PlayFromStart`)
      (:`Update`
        (`SceneComponent.K2_SetRelativeRotation` (`self.SM_Door`) (`KismetMathLibrary.RLerp` (`BlueprintMapLibrary.Map_Find` (`self.TargetRotationByState`) (`self.State`)) (`BlueprintMapLibrary.Map_Find` (`self.TargetRotationByState`) TargetState) _newtrack_0) false false)
        (`/Engine/EditorBlueprintResources/StandardMacros.DoOnce` false
          (:`Completed`
            (set `self.bTransitioning` true))))
      (:`Finished`
        (set `self.State` (`self.TargetState`))
        (set `self.bTransitioning` false)
        (if (`self.bStateQueued`)
          (`self.TransitionToState` (`self.QueuedTargetState`)))))
    (else
      (set `self.TargetState` TargetState)
      (set `self.bStateQueued` true))))

(fn `UserConstructionScript`
  (`SceneComponent.K2_SetRelativeRotation` (`self.SM_Door`) (`BlueprintMapLibrary.Map_Find` (`self.TargetRotationByState`) (`self.State`)) false false))
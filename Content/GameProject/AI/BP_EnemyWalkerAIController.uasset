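; AI controller for walker enemies that runs their behavior tree and tracks the player through AI perception.
; On possession it starts BT_EnemyWalker.
; Perception updates store player character 0 in the TargetPlayer blackboard key when sensed.
; Any other update, including one for a different actor, clears that key.
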(event `self.ReceivePossess`
  (params (PossessedPawn :type "Pawn Object Reference"))
  (`self.RunBehaviorTree` "/Game/GameProject/AI/BT_EnemyWalker.BT_EnemyWalker"))

(event `self.AIPerception.OnTargetPerceptionUpdated`
  (params (Actor :type "Actor Object Reference") (Stimulus :type "AIStimulus Structure"))
  (bind _blackboard (`self.Blackboard`))
  (if (and (== Actor (`GameplayStatics.GetPlayerCharacter` 0)) (`.bSuccessfullySensed` (break `AIStimulus` Stimulus)))
    (`BlackboardComponent.SetValueAsObject` _blackboard "TargetPlayer" Actor)
    (else
      (`BlackboardComponent.SetValueAsObject` _blackboard "TargetPlayer" null))))

(fn `UserConstructionScript`)
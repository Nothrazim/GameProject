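; AI controller for the flyer enemy that runs the BT_EnemyWalker behavior tree on possess.
; Its AI Perception update event is unwired, so the player-sensing logic never runs.
; That disconnected logic would set HasLineOfSight and EnemyActor on the Blackboard when a Player-tagged actor is sensed.
; Otherwise it would start a timer that clears both keys after a line-of-sight delay.
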(event `self.ReceivePossess`
  (params (PossessedPawn :type "Pawn Object Reference"))
  (`self.RunBehaviorTree` "/Game/GameProject/AI/BT_EnemyWalker.BT_EnemyWalker"))

(event `self.AIPerception.OnTargetPerceptionUpdated`
  (params (Actor :type "Actor Object Reference") (Stimulus :type "AIStimulus Structure"))
  ;[1 1 1] AI Perception, setting HasLineOfSight to true if detected or to false if losing track of player
)

(event `StartEnemyTimer`
  (bind _blackboard (`self.Blackboard`))
  ;[1 1 1] AI Perception, setting HasLineOfSight to true if detected or to false if losing track of player
  (`BlackboardComponent.SetValueAsBool` _blackboard (`self.HasLineOfSight`) false)
  (`BlackboardComponent.SetValueAsObject` _blackboard (`self.EnemyActor`) null)
  (`KismetSystemLibrary.PrintString` "Where did you go?"))

(fn `UserConstructionScript`)